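; BP_ky_fireTrail is a self-destroying magic effect actor that animates three fire trails around a rotating Scene pivot.
; On BeginPlay, chained timelines spin the pivot, offset it vertically while its Z exceeds 50, and shift the trails along local X while Trail1's X exceeds 50.
; Once that X threshold is no longer exceeded, the trails snap to a fixed relative position and the actor is destroyed after a short delay.
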(event EventBeginPlay
  (bind _scene (Variables|Default|GetScene))
  (bind _trail1 (Variables|Default|Gettrail1))
  (bind _rotation (Timeline|Timeline_0 Play)
    (:Update
      (Transformation|AddLocalRotation (Variables|Default|GetScene) (Math|Rotator|MakeRotator 0.0 0.0 (* _rotation (stale EventTick DeltaSeconds))) false false)
      (if (> (.z (Variables|/Script/Engine.SceneComponent|GetRelativeLocation _scene)) 5e+01)
        (bind _float (Timeline|Timeline_2 Play)
          (:Update
            (Transformation|AddLocalOffset (Variables|Default|GetScene) (Math|Vector|MakeVector 0.0 0.0 (* _float (stale EventTick DeltaSeconds))) false false)))
        (else
          (Transformation|SetRelativeLocation _scene (Math|Vector|MakeVector 0.0 0.0 0.0) false false)))
      (if (> (.x (Variables|/Script/Engine.SceneComponent|GetRelativeLocation _trail1)) 5e+01)
        (bind _location (Timeline|Timeline_1 Play)
          (:Update
            (Transformation|AddLocalOffset _trail1 (Math|Vector|MakeVector (* _location (stale EventTick DeltaSeconds)) 0.0 0.0) false false)))
        (else
          (Transformation|SetRelativeLocation _trail1 (Math|Vector|MakeVector 0.0 0.0 5e+01) false false)
          (Utilities|FlowControl|Delay 1.0)
          (Actor|DestroyActor))))))

(event Collision|EventActorBeginOverlap
  (params (OtherActor :type Actor%20Object%20Reference)))

(event EventTick
  (params (DeltaSeconds :type Float%20%28single-precision%29)))

(fn ConstructionScript)